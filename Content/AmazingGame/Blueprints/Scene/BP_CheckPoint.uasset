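; BP_CheckPoint is a checkpoint that saves the player's respawn point when BP_MainCharacter's root component overlaps its capsule.
; On the first such overlap only, it converts the linked PlayerStart's tag to an integer and stores it as SpawnPlayerIndex on BP_MyGameMode.
; It then plays a timeline that drives the Alpha material parameter on its rune pillar mesh as visual activation feedback.
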(event OnComponentBeginOverlap(Capsule)
  (params (OverlappedComponent :type Primitive%20Component%20Object%20Reference) (OtherActor :type Actor%20Object%20Reference) (OtherComp :type Primitive%20Component%20Object%20Reference) (OtherBodyIndex :type Integer) (bFromSweep :type Boolean) (SweepResult :type Hit%20Result%20Structure%20%28by%20ref%29))
  (bind _asbp_main_character (Utilities|Casting|CastToBP_MainCharacter OtherActor))
  (if (== (Variables|/Script/Engine.Actor|GetRootComponent _asbp_main_character) OtherComp)
    (Utilities|FlowControl|DoOnce false
      (:Completed
        (Utilities|FlowControl|Sequence
          (:then_0
            (bind _asbp_my_game_mode (Utilities|Casting|CastToBP_MyGameMode (Game|GetGameMode)))
            (Variables|/Game/AmazingGame/Blueprints/GameMode/BP_MyGameMode.BP_MyGameMode_C|SetSpawnPlayerIndex _asbp_my_game_mode (Math|Conversions|ToInteger(Byte) (Utilities|String|ToString(Name) (Variables|/Script/Engine.PlayerStart|GetPlayerStartTag (Variables|Default|GetPlayerStart))))))
          (:then_1
            (bind _alpha (Timeline|TimelineEffect PlayFromStart)
              (:Update
                (Rendering|Material|SetScalarParameterValueonMaterials (Variables|Default|GetSM_Env_Rune_Pillar_03) "Alpha" _alpha)))))))))

(fn ConstructionScript)