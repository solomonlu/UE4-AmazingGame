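; BP_FireWall is a fire wall hazard that burns characters and can be put out by a water spirit's attack ball.
; A Tick-driven one-second Delay periodically applies fixed damage to every Character overlapping DamageBox.
; The first BP_WaterSpirit_AttackBall to enter the box is destroyed and starts a timeline that animates the particle Spawn parameter, then destroys the wall.
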(event OnComponentBeginOverlap(DamageBox)
  (params (OverlappedComponent :type Primitive%20Component%20Object%20Reference) (OtherActor :type Actor%20Object%20Reference) (OtherComp :type Primitive%20Component%20Object%20Reference) (OtherBodyIndex :type Integer) (bFromSweep :type Boolean) (SweepResult :type Hit%20Result%20Structure%20%28by%20ref%29))
  (Utilities|Casting|CastToBP_WaterSpirit_AttackBall OtherActor)
  (Utilities|FlowControl|DoOnce false
    (:Completed
      (Actor|DestroyActor OtherActor)
      (bind _lerp (Timeline|TimelineDisappear PlayFromStart)
        (:Update
          (Effects|Components|ParticleSystem|SetFloatParameter (Variables|Default|GetP_file) "Spawn" _lerp))
        (:Finished
          (Actor|DestroyActor))))))

(event EventTick
  (params (DeltaSeconds :type Float%20%28single-precision%29))
  (Utilities|FlowControl|Delay 1.0)
  (for _array_element (Collision|GetOverlappingActors (Variables|Default|GetDamageBox) "/Script/Engine.Character" :!class /Script/Engine.PrimitiveComponent)
    (Game|Damage|ApplyDamage _array_element 1e+01 0 self)))

(fn ConstructionScript)