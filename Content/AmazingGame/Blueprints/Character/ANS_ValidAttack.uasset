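; Anim notify state that marks the attack-valid window in the main character's animations.
; On begin, it casts the mesh owner to BP_MainCharacter and sets its ValidAttack flag to true.
; On end, it does the same cast and sets the flag back to false.
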(fn ReceivedNotifyBegin
  (params (MeshComp :type Skeletal%20Mesh%20Component%20Object%20Reference) (Animation :type Anim%20Sequence%20Base%20Object%20Reference) (TotalDuration :type Float%20%28single-precision%29))
  (bind _asbp_main_character (Utilities|Casting|CastToBP_MainCharacter (Components|GetOwner MeshComp))
    (:then
      (Default|SetValidAttack _asbp_main_character true)
      (return true))
    (:CastFailed
      (return true))))

(fn ReceivedNotifyEnd
  (params (MeshComp :type Skeletal%20Mesh%20Component%20Object%20Reference) (Animation :type Anim%20Sequence%20Base%20Object%20Reference))
  (bind _asbp_main_character (Utilities|Casting|CastToBP_MainCharacter (Components|GetOwner MeshComp))
    (:then
      (Default|SetValidAttack _asbp_main_character false)
      (return true))
    (:CastFailed
      (return true))))