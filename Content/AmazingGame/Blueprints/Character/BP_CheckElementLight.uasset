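; BP_CheckElementLight is an actor that detects the element of what it hits and spawns a spirit-change ball for the matching spirit.
; On its first hit it sets a short lifespan and checks the other actor for a Water, Fire or Shadow tag.
; If the game mode reports that spirit category unlocked, it spawns BP_ChangeSpiritBall at its own transform, set to that category.
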(event Collision|EventHit
  (params (MyComp :type Primitive%20Component%20Object%20Reference) (Other :type Actor%20Object%20Reference) (OtherComp :type Primitive%20Component%20Object%20Reference) (bSelfMoved :type Boolean) (HitLocation :type Vector :default "0, 0, 0") (HitNormal :type Vector :default "0, 0, 0") (NormalImpulse :type Vector :default "0, 0, 0") (Hit :type Hit%20Result%20Structure%20%28by%20ref%29))
  (bind _returnvalue (Transformation|GetActorRotation))
  (bind _returnvalue_2 (Transformation|GetActorLocation))
  (Utilities|FlowControl|DoOnce false
    (:Completed
      (Actor|SetLifeSpan 0.1)
      (Utilities|CheckActorTag Other
        (:Water
          (if (CallFunction|CheckSpiritUnlock "NewEnumerator1")
            (Game|SpawnActorfromClass "/Game/AmazingGame/Blueprints/Character/BP_ChangeSpiritBall.BP_ChangeSpiritBall_C" (Math|Transform|MakeTransform _returnvalue_2 _returnvalue "1,1,1") "Undefined" 0 "NewEnumerator1" 0)))
        (:Fire
          (if (CallFunction|CheckSpiritUnlock "NewEnumerator2")
            (Game|SpawnActorfromClass "/Game/AmazingGame/Blueprints/Character/BP_ChangeSpiritBall.BP_ChangeSpiritBall_C" (Math|Transform|MakeTransform _returnvalue_2 _returnvalue "1,1,1") "Undefined" 0 "NewEnumerator2" 0)))
        (:Shadow
          (if (CallFunction|CheckSpiritUnlock "NewEnumerator3")
            (Game|SpawnActorfromClass "/Game/AmazingGame/Blueprints/Character/BP_ChangeSpiritBall.BP_ChangeSpiritBall_C" (Math|Transform|MakeTransform _returnvalue_2 _returnvalue "1,1,1") "Undefined" 0 "NewEnumerator3" 0)))))))

(fn ConstructionScript)

(fn CheckSpiritUnlock
  (params (SpiritCategory :type ESpiritCategory%20Enum :default "NewEnumerator0"))
  (return (Default|IsSpiritUnlocked (.AsBP%20My%20Game%20Mode (Utilities|Casting|CastToBP_MyGameMode (Game|GetGameMode))) SpiritCategory)))