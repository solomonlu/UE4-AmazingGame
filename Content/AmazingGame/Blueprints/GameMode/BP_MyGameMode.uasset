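; BP_MyGameMode is a game mode that picks player start points and tracks which spirits are unlocked.
; FindPlayerStart returns a PlayerStart whose tag matches SpawnPlayerIndex, falling back to the first one found if LocalPlayerStart is invalid.
; The UnlockSpirit event adds unique entries to UnlockedSpirits, which IsSpiritUnlocked searches to report whether a spirit category is available.
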(event Custom|UnlockSpirit
  (params (UnlockSpirit :type ESpiritCategory%20Enum :default "NewEnumerator0"))
  (Utilities|Array|AddUnique (Variables|Default|GetUnlockedSpirits) UnlockSpirit))

(fn ConstructionScript)

(fn FindPlayerStart
  (params (Player :type Controller%20Object%20Reference) (IncomingName :type String))
  (bind _outactors (Actor|GetAllActorsOfClass "/Script/Engine.PlayerStart"))
  (for _array_element _outactors
    (if (Utilities|Name|Equal(Name) (Variables|/Script/Engine.PlayerStart|GetPlayerStartTag _array_element) (Utilities|String|StringToName (Utilities|String|ToString(Integer) (Variables|Default|GetSpawnPlayerIndex))))
      (LocalVariables|SetLocalPlayerStart _array_element)))
  (Utilities|IsValid (LocalVariables|GetLocalPlayerStart)
    (:Is%20Valid
      (return (LocalVariables|GetLocalPlayerStart)))
    (:Is%20Not%20Valid
      (return (Utilities|Array|Get(acopy) _outactors)))))

(fn IsSpiritUnlocked
  (params (SpiritCategory :type ESpiritCategory%20Enum :default "NewEnumerator0"))
  (return (not (== (Utilities|Array|FindItem (Variables|Default|GetUnlockedSpirits) SpiritCategory) -1))))