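; Base NPC actor that turns to face the nearby player and shows table-driven dialog when interacted with.
; On BeginPlay it caches DT_Dialog rows matching its NPCName, and sphere overlaps register it as the main character's interactable.
; Each Interact advances the line and shows the text matching ConversationID and line number in a dialog widget.
; Leaving the sphere or lacking exactly one matching line clears the dialog and resets the counter.
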(event OnComponentBeginOverlap(CheckPlayerSphere)
  (params (OverlappedComponent :type Primitive%20Component%20Object%20Reference) (OtherActor :type Actor%20Object%20Reference) (OtherComp :type Primitive%20Component%20Object%20Reference) (OtherBodyIndex :type Integer) (bFromSweep :type Boolean) (SweepResult :type Hit%20Result%20Structure%20%28by%20ref%29))
  (bind _asbp_main_character (Utilities|Casting|CastToBP_MainCharacter OtherActor))
  (bind _output_get (Variables|Default|SetMainCharacterRef _asbp_main_character))
  (Default|SetIntactableActor _output_get self))

(event OnComponentEndOverlap(CheckPlayerSphere)
  (params (OverlappedComponent :type Primitive%20Component%20Object%20Reference) (OtherActor :type Actor%20Object%20Reference) (OtherComp :type Primitive%20Component%20Object%20Reference) (OtherBodyIndex :type Integer))
  (bind _asbp_main_character (Utilities|Casting|CastToBP_MainCharacter OtherActor))
  (Default|UnsetIntactableActor _asbp_main_character)
  (Variables|Default|SetMainCharacterRef 0)
  (CallFunction|ClearDialog))

(event EventTick
  (params (DeltaSeconds :type Float%20%28single-precision%29))
  (Utilities|IsValid (Variables|Default|GetMainCharacterRef)
    (:Is%20Valid
      (Transformation|SetActorRotation (Math|Rotator|FindLookatRotation (Transformation|GetActorLocation) (Transformation|GetActorLocation (Variables|Default|GetMainCharacterRef)))))))

(event EventInteract
  (bind (_dialogexist _currentdialogtext) (CallFunction|DialogGetLine))
  (bind (_dialogexist_2 _currentdialogtext_2) (CallFunction|DialogGetLine))
  ;[1 1 1] Dialog
  (Math|Integer|IncrementInt (Variables|Dialog|GetCurrentLine)
    (:%20%20
      (Utilities|IsValid (Variables|Dialog|GetDialogWidgetRef)
        (:Is%20Valid
          (if _dialogexist_2
            (Variables|/Game/AmazingGame/Blueprints/UMG/InGame/UMG_InGame_Dialog.UMG_InGame_Dialog_C|SetDialogText (Variables|Dialog|GetDialogWidgetRef) _currentdialogtext_2)))
        (:Is%20Not%20Valid
          (bind _returnvalue (UserInterface|CreateWidget "/Game/AmazingGame/Blueprints/UMG/InGame/UMG_InGame_Dialog.UMG_InGame_Dialog_C" (Game|GetPlayerController 0)))
          (bind _output_get (Variables|Dialog|SetDialogWidgetRef _returnvalue))
          (UserInterface|Viewport|AddtoViewport _output_get 0)
          (if _dialogexist
            (Variables|/Game/AmazingGame/Blueprints/UMG/InGame/UMG_InGame_Dialog.UMG_InGame_Dialog_C|SetDialogText _output_get _currentdialogtext)))))))

(event EventBeginPlay
  ;[1 1 1] Dialog
  (bind _outrownames (DataTable|GetDataTableRowNames "/Game/AmazingGame/Blueprints/NPC/Dialog/DT_Dialog.DT_Dialog"))
  (for _array_element _outrownames
    (bind _returnvalue (Utilities|GetDataTableRow "/Game/AmazingGame/Blueprints/NPC/Dialog/DT_Dialog.DT_Dialog" _array_element)
      (:then
        (if (Utilities|Enum|Equal(Enum) (.NPC_Name (Utilities|Struct|BreakSTR_Dialog _returnvalue)) (Variables|Default|GetNPC_Name))
          (Utilities|Array|Add (Variables|Dialog|GetMyDialogRows) _array_element))))))

(fn ConstructionScript)

(fn DialogGetLine
  (for _array_element (Variables|Dialog|GetMyDialogRows)
    (bind _returnvalue (Utilities|GetDataTableRow "/Game/AmazingGame/Blueprints/NPC/Dialog/DT_Dialog.DT_Dialog" _array_element)
      (:then
        (if (and (== (.Conversation_ID (Utilities|Struct|BreakSTR_Dialog _returnvalue)) (Variables|Dialog|GetConversationID)) (== (.Line_ID (Utilities|Struct|BreakSTR_Dialog _returnvalue)) (Variables|Dialog|GetCurrentLine)))
          (Utilities|Array|Add (LocalVariables|GetLocalDialogTexts) (.Dialog_Text (Utilities|Struct|BreakSTR_Dialog _returnvalue)))))))
  (if (== (Utilities|Array|Length (LocalVariables|GetLocalDialogTexts)) 1)
    (return true (Utilities|Array|Get(acopy) (LocalVariables|GetLocalDialogTexts)))
    (else
      (CallFunction|ClearDialog)
      (return false ""))))

(fn ClearDialog
  (Variables|Dialog|SetCurrentLine 0)
  (Utilities|IsValid (Variables|Dialog|GetDialogWidgetRef)
    (:Is%20Valid
      (Widget|RemovefromParent (Variables|Dialog|GetDialogWidgetRef))
      (Variables|Dialog|SetDialogWidgetRef 0))))