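; BP_PoisonCloud is a Necrolyte boss hazard that can be lobbed to a location and damages the player inside it.
; FlyTo solves an arcing toss velocity from a fixed launch speed and the projectile's gravity scale, then activates ProjectileMovement.
; From BeginPlay, a looping one-second timer applies fixed damage to every BP_MainCharacter overlapping the Box, regardless of whether the cloud has landed.
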(event Custom|FlyTo
  (params (Location :type Vector))
  (bind _tossvelocity (Class|GameplayStatics|BlueprintSuggestProjectileVelocity (Transformation|GetActorLocation) Location 6e+02 (* (Variables|/Script/Engine.ProjectileMovementComponent|GetProjectileGravityScale (Variables|Default|GetProjectileMovement)) -9.8e+02) "DoNotTrace" 0.0 false false))
  (Variables|/Script/Engine.MovementComponent|SetVelocity (Variables|Default|GetProjectileMovement) _tossvelocity)
  (Components|Activation|SetActive (Variables|Default|GetProjectileMovement) true false))

(event Custom|CheckPlayerInCloud
  (for _array_element (Collision|GetOverlappingActors (Variables|Default|GetBox) "/Game/AmazingGame/Blueprints/Character/BP_MainCharacter.BP_MainCharacter_C" :!class /Script/Engine.PrimitiveComponent)
    (Game|Damage|ApplyDamage _array_element 1e+01 0 0)))

(event EventBeginPlay
  (Utilities|Time|SetTimerbyFunctionName 0 "CheckPlayerInCloud" 1.0 true))

(fn ConstructionScript)