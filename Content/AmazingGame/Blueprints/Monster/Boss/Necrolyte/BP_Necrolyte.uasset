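; Necrolyte boss that, once activated, faces the player and loops through randomly chosen spells until death, when it ragdolls.
; Montage notifies drive poison clouds launched around the player, staggered skeleton summons, or a bone cage that chains into Death Finger.
; It is invulnerable while casting, and each montage completion re-enables damage and leads to the next skill.
; Damage triggers a directional hit reaction, then a teleport to a navigable point near the player.
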(event Custom|CastPoisonCloud
  (|CastPoisonCloudNode))

(event Custom|CastSkeletonArmy
  (|CastSkeletonArmyNode))

(event Custom|CastBoneCage
  (|CastBoneCageNode))

(event Custom|CastDeathFinger
  (|CastDeathFingerNode))

(event Custom|DesideWhatSkill
  (if (not (Variables|Default|GetIsDeath))
    (switch int (Math|Random|RandomIntegerinRange 0 2)
      (:0
        (CallFunction|CastPoisonCloud))
      (:1
        (CallFunction|CastSkeletonArmy))
      (:2
        (CallFunction|CastBoneCage)))))

(event EventTick
  (params (DeltaSeconds :type Float%20%28single-precision%29))
  (|AlwaysLookAtPlayer))

(event EventOnDeath
  (bind _capsulecomponent (Variables|Default|GetCapsuleComponent))
  (bind _mesh (Variables|Character|GetMesh))
  (Variables|Default|SetIsDeath true)
  (Collision|SetCollisionResponsetoAllChannels _capsulecomponent "ECR_Ignore")
  (Collision|SetCollisionResponsetoChannel _capsulecomponent "ECC_WorldStatic" "ECR_Block")
  (Collision|SetCollisionProfileName _mesh "Ragdoll" :!class /Script/Engine.PrimitiveComponent)
  (Physics|SetSimulatePhysics _mesh true))

(event EventOnDamaged
  (params (Damage :type Float%20%28single-precision%29) (DamageCauser :type Actor%20Object%20Reference))
  (bind _mesh (Variables|Character|GetMesh))
  (Utilities|FlowControl|Sequence
    (:then_0
      (bind _returnvalue (Class|AnimInstance|CalculateDirection (Components|SkeletalMesh|GetAnimInstance (Variables|Character|GetMesh)) (Math|Transform|InverseTransformDirection (Transformation|GetActorTransform) (- (Transformation|GetActorLocation) (Transformation|GetActorLocation DamageCauser))) (Transformation|GetActorRotation)))
      (Utilities|CalcDirection _returnvalue
        (:Front
          (Animation|Montage|PlayMontage _mesh "/Game/Art/polygon/monster/MageAnimset/Mage_Hit_Reaction_Front_04_Montage.Mage_Hit_Reaction_Front_04_Montage"))
        (:Left
          (Animation|Montage|PlayMontage _mesh "/Game/Art/polygon/monster/MageAnimset/Mage_Hit_Reaction_Left_01_Montage.Mage_Hit_Reaction_Left_01_Montage"))
        (:Right
          (Animation|Montage|PlayMontage _mesh "/Game/Art/polygon/monster/MageAnimset/Mage_Hit_Reaction_Right_01_Montage.Mage_Hit_Reaction_Right_01_Montage"))
        (:Back
          (Animation|Montage|PlayMontage _mesh "/Game/Art/polygon/monster/MageAnimset/Mage_Hit_Reaction_Back_01_Montage.Mage_Hit_Reaction_Back_01_Montage"))))
    (:then_2
      (Utilities|FlowControl|Delay 0.5)
      (Transformation|Teleport (CallFunction|CalcLocationAroundPlayer 2e+03 1.5e+03) "0, 0, 0"))))

(event EventActive
  (Variables|Default|SetIsActived true)
  (Utilities|FlowControl|Delay 5.0)
  (CallFunction|DesideWhatSkill))

(event EventBeginPlay
  (Utilities|FlowControl|Sequence
    (:then_1
      (bind _outactors (Actor|GetAllActorsOfClass "/Game/AmazingGame/Blueprints/Character/BP_MainCharacter.BP_MainCharacter_C"))
      (Variables|Default|SetMainCharacterRef (Utilities|Array|Get(acopy) _outactors)))))

(fn ConstructionScript
  (|CallParentFunction))

(fn CalcLocationAroundPlayer
  (params (Radius :type Float%20%28single-precision%29) (KeepDistance :type Float%20%28single-precision%29))
  (LocalVariables|SetResultLocation (.RandomLocation (Class|NavigationSystemV1|GetRandomPointinNavigableRadius (Transformation|GetActorLocation (Variables|Default|GetMainCharacterRef)) Radius 0 0)))
  (while (> (Math|Vector|VectorLength (- (Transformation|GetActorLocation (Variables|Default|GetMainCharacterRef)) (LocalVariables|GetResultLocation))) KeepDistance)
    (LocalVariables|SetResultLocation (.RandomLocation (Class|NavigationSystemV1|GetRandomPointinNavigableRadius (Transformation|GetActorLocation (Variables|Default|GetMainCharacterRef)) Radius 0 0))))
  (return (LocalVariables|GetResultLocation)))