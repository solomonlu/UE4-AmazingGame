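; Necrolyte boss bone cage that roots the player character in place until the cage is destroyed.
; The first main character to overlap its sphere has their max walk speed saved and set to zero, guarded by a DoOnce.
; On Destroyed, it writes the saved speed back to that character, without checking that one was ever caught.
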(event OnComponentBeginOverlap(Sphere)
  (params (OverlappedComponent :type Primitive%20Component%20Object%20Reference) (OtherActor :type Actor%20Object%20Reference) (OtherComp :type Primitive%20Component%20Object%20Reference) (OtherBodyIndex :type Integer) (bFromSweep :type Boolean) (SweepResult :type Hit%20Result%20Structure%20%28by%20ref%29))
  (bind _asbp_main_character (Utilities|Casting|CastToBP_MainCharacter OtherActor))
  (Utilities|FlowControl|DoOnce false
    (:Completed
      (Variables|Default|SetMainCharacterRef _asbp_main_character)
      (Variables|Default|SetRestoreSpeed (Variables|/Script/Engine.CharacterMovementComponent|GetMaxWalkSpeed (Variables|/Script/Engine.Character|GetCharacterMovement _asbp_main_character)))
      (Variables|/Script/Engine.CharacterMovementComponent|SetMaxWalkSpeed (Variables|/Script/Engine.Character|GetCharacterMovement _asbp_main_character) 0.0))))

(event EventDestroyed
  (Variables|/Script/Engine.CharacterMovementComponent|SetMaxWalkSpeed (Variables|/Script/Engine.Character|GetCharacterMovement (Variables|Default|GetMainCharacterRef)) (Variables|Default|GetRestoreSpeed)))

(fn ConstructionScript)