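; BP_BigSpider is a spider boss that fights the main character with randomly chosen skills.
; A self-repeating, delayed skill picker runs a melee approach with random montages, a charge, or a summon of small spiders on a montage notify.
; Capsule overlaps during a charge, confirmed by the melee collision, deal damage and knockback, gated by a DoOnce reset each charge.
; Death stops the picker, unpossesses the controller, ragdolls the mesh and sets a lifespan.
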(event OnComponentBeginOverlap(CapsuleComponent)
  (params (OverlappedComponent :type Primitive%20Component%20Object%20Reference) (OtherActor :type Actor%20Object%20Reference) (OtherComp :type Primitive%20Component%20Object%20Reference) (OtherBodyIndex :type Integer) (bFromSweep :type Boolean) (SweepResult :type Hit%20Result%20Structure%20%28by%20ref%29))
  (if (Variables|Default|GetIsInCharging)
    (bind _asbp_main_character (Utilities|Casting|CastToBP_MainCharacter OtherActor))
    (if (Collision|IsOverlappingActor (Variables|Default|GetMeleeCollision) _asbp_main_character :!class /Script/Engine.PrimitiveComponent)
      (Utilities|FlowControl|DoOnce true
        (:Completed
          (Game|Damage|ApplyDamage _asbp_main_character 5e+01 0 self)
          (Character|LaunchCharacter _asbp_main_character (Math|Vector|MakeVector (.x (* (Math|Vector|Normalize (- (Transformation|GetActorLocation _asbp_main_character) (Transformation|GetActorLocation))) 1e+03)) (.y (* (Math|Vector|Normalize (- (Transformation|GetActorLocation _asbp_main_character) (Transformation|GetActorLocation))) 1e+03)) 5e+02) false false))))))

(event Custom|CastMeleeAttack
  (Transformation|SetActorRotation (Math|Rotator|FindLookatRotation (Transformation|GetActorLocation) (Transformation|GetActorLocation (Variables|Default|GetMainCharacterRef))))
  (AI|AIMoveTo (.AsAIController (Utilities|Casting|CastToAIController (Pawn|GetController))) "0, 0, 0" (Variables|Default|GetMainCharacterRef) 5e+01 "Default" "Default" true true
    (:OnMoveFinished
      (Animation|Montage|PlayMontage (Variables|Character|GetMesh) (Utilities|Select :Index (Math|Random|RandomIntegerinRange 0 2) :Option%200 "/Game/Art/anim/zhizhu/Animation/ExoGame_Greater_Spider_Attack_Melee_B_Montage.ExoGame_Greater_Spider_Attack_Melee_B_Montage" :Option%201 "/Game/Art/anim/zhizhu/Animation/ExoGame_Greater_Spider_Attack_Melee_C_Montage.ExoGame_Greater_Spider_Attack_Melee_C_Montage" :Option%202 "/Game/Art/anim/zhizhu/Animation/ExoGame_Greater_Spider_Attack_Melee_Montage.ExoGame_Greater_Spider_Attack_Melee_Montage")))))

(event Custom|CastCharge
  (Transformation|SetActorRotation (Math|Rotator|FindLookatRotation (Transformation|GetActorLocation) (Transformation|GetActorLocation (Variables|Default|GetMainCharacterRef))))
  (Animation|Montage|PlayMontage (Variables|Character|GetMesh) "/Game/Art/anim/zhizhu/Animation/ExoGame_Greater_Spider_Charge_Montage.ExoGame_Greater_Spider_Charge_Montage"
    (:then
      (Variables|Default|SetIsInCharging true)
      (CallFunction|ResetCharge))
    (:OnCompleted
      (Variables|Default|SetIsInCharging false))))

(event Custom|CastSummon
  (Transformation|SetActorRotation (Math|Rotator|FindLookatRotation (Transformation|GetActorLocation) (Transformation|GetActorLocation (Variables|Default|GetMainCharacterRef))))
  (bind _notifyname (Animation|Montage|PlayMontage (Variables|Character|GetMesh) "/Game/Art/anim/zhizhu/Animation/ExoGame_Greater_Spider_Cast_Summon_Montage.ExoGame_Greater_Spider_Cast_Summon_Montage")
    (:OnNotifyBegin
      (if (Utilities|Name|Equal(Name) _notifyname "SummonSpiders")
        (for _index (range 0 2)
          (Game|SpawnActorfromClass "/Game/AmazingGame/Blueprints/Monster/Boss/BigSpider/BP_SmallSpider.BP_SmallSpider_C" (Math|Transform|MakeTransform (Transformation|GetActorLocation) (Transformation|GetActorRotation) "1,1,1") "AdjustIfPossibleButAlwaysSpawn" 0 0))))))

(event Custom|ResetCharge
  (Utilities|FlowControl|DoOnce true) ; enters at Reset
)

(event Custom|DesideWhatSkill
  (if (not (Variables|Default|GetIsDeath))
    (switch int (Math|Random|RandomIntegerinRange 0 2)
      (:0
        (CallFunction|CastMeleeAttack))
      (:1
        (CallFunction|CastCharge))
      (:2
        (CallFunction|CastSummon)))
    (Utilities|FlowControl|Delay 5.0)
    (CallFunction|DesideWhatSkill)))

(event EventOnDeath
  (bind _returnvalue (Pawn|GetController))
  (bind _capsulecomponent (Variables|Default|GetCapsuleComponent))
  (bind _mesh (Variables|Character|GetMesh))
  (Variables|Default|SetIsDeath true)
  (Actor|SetLifeSpan 15.0)
  (if (Utilities|IsValid _returnvalue)
    (Pawn|UnPossess _returnvalue)
    (Collision|SetCollisionResponsetoAllChannels (Variables|Default|GetMeleeCollision) "ECR_Ignore")
    (Collision|SetCollisionResponsetoAllChannels _capsulecomponent "ECR_Ignore")
    (Collision|SetCollisionResponsetoChannel _capsulecomponent "ECC_WorldStatic" "ECR_Block")
    (Collision|SetCollisionProfileName _mesh "Ragdoll" :!class /Script/Engine.PrimitiveComponent)
    (Physics|SetSimulatePhysics _mesh true)))

(event EventActive
  (Variables|Default|SetIsActived true))

(event EventBeginPlay
  (bind _outactors (Actor|GetAllActorsOfClass "/Game/AmazingGame/Blueprints/Character/BP_MainCharacter.BP_MainCharacter_C"))
  (Variables|Default|SetMainCharacterRef (Utilities|Array|Get(acopy) _outactors)))

(fn ConstructionScript)