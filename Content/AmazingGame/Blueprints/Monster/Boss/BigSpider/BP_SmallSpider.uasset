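; BP_SmallSpider is a small spider monster from the Big Spider boss set that defines how it reacts to damage and death.
; Taking damage plays a heavy front-hit reaction montage.
; On death it sets a delayed despawn, then, if a controller is valid, unpossesses, disables melee collision and notifies its behavior component.
; That same branch pushes the mesh bodies from the root away from the damage causer with an impulse.
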(event EventOnDeath
  (bind _returnvalue (Pawn|GetController))
  (Actor|SetLifeSpan 15.0)
  (if (Utilities|IsValid _returnvalue)
    (Pawn|UnPossess _returnvalue)
    (Collision|SetCollisionResponsetoAllChannels (Variables|Default|GetMeleeCollision) "ECR_Ignore")
    (Default|OnDeath (Variables|Default|GetBP_BehaviorComponent))
    (Class|SkeletalMeshComponent|AddImpulsetoAllBodiesBelow (Variables|Character|GetMesh) (* (Math|Vector|Normalize (- (Transformation|GetActorLocation) (Transformation|GetActorLocation (Variables|Default|GetDamageCauser)))) 1e+03) "root" false true)))

(event EventOnDamaged
  (params (Damage :type Float%20%28single-precision%29) (DamageCauser :type Actor%20Object%20Reference))
  (Animation|Montage|PlayMontage (Variables|Character|GetMesh) "/Game/Art/anim/zhizhu/Animation/ExoGame_Greater_Spider_React_Heavy_Front_Montage.ExoGame_Greater_Spider_React_Heavy_Front_Montage"))

(fn ConstructionScript
  (|CallParentFunction))