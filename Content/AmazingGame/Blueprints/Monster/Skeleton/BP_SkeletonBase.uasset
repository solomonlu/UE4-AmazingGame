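; Base skeleton monster that handles spawn poses, AI startup, hit reactions and death.
; Grave, sitting and laying states pass to the anim Blueprint, while the None state runs SpawnEnd immediately.
; SpawnEnd enables damage, adds behavior components with the generic AI tree and spawns a possessing AI controller.
; Damage notifies the behavior component and plays a directional hit montage; death adds particles, unpossesses and pushes the mesh bodies away from the damage causer.
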(event Custom|SpawnEnd
  ;[0 0.3233 1] Spawn Event
  (Variables|Default|SetbCanBeDamaged true)
  (bind _returnvalue (AddComponent|AddBPBehaviorComponent :PatrolRoute 0 :SeekTarget 0 :BehaviorTree "/Game/AIBehaviorToolkit/Blueprints/BehaviorTree/BT_GenericAI.BT_GenericAI"))
  (Variables|Default|SetBP_BehaviorComponent _returnvalue)
  (AddComponent|AddBPBehaviorTriggerComponent)
  (bind _returnvalue_2 (Game|SpawnActorfromClass "/Game/AIBehaviorToolkit/Blueprints/BP_AIC.BP_AIC_C" (Transformation|GetActorTransform) "Undefined" 0 0))
  (Pawn|Possess _returnvalue_2 self))

(event EventBeginPlay
  ;[0 0.3233 1] Spawn Event
  (switch Utilities|FlowControl|Switch|SwitchonESkeletonInitState (Variables|Default|GetInitState)
    (:NewEnumerator0
      (bind _asbpa_skeleton (Utilities|Casting|CastToBPA_Skeleton (Components|SkeletalMesh|GetAnimInstance (Variables|Character|GetMesh))))
      (Variables|/Game/AmazingGame/Blueprints/Monster/Skeleton/BPA_Skeleton.BPA_Skeleton_C|SetIsSpawnEnd _asbpa_skeleton true)
      (CallFunction|SpawnEnd))
    (:NewEnumerator1
      (bind _asbpa_skeleton_2 (Utilities|Casting|CastToBPA_Skeleton (Components|SkeletalMesh|GetAnimInstance (Variables|Character|GetMesh)) :!label _label))
      (Variables|/Game/AmazingGame/Blueprints/Monster/Skeleton/BPA_Skeleton.BPA_Skeleton_C|SetInitState _asbpa_skeleton_2 (Variables|Default|GetInitState))
      (Variables|/Game/AmazingGame/Blueprints/Monster/Skeleton/BPA_Skeleton.BPA_Skeleton_C|SetIsActive _asbpa_skeleton_2 (Variables|Default|GetIsActive)))
    (:NewEnumerator2
      (goto _label))
    (:NewEnumerator3
      (goto _label))))

(event EventOnDeath
  (bind _returnvalue (Pawn|GetController))
  ;[1 0.9532 0.1043] Damage Event
  (AddComponent|AddParticleSystemComponent false)
  (if (Utilities|IsValid _returnvalue)
    (Pawn|UnPossess _returnvalue)
    (Default|OnDeath (Variables|Default|GetBP_BehaviorComponent))
    (Class|SkeletalMeshComponent|AddImpulsetoAllBodiesBelow (Variables|Character|GetMesh) (* (Math|Vector|Normalize (- (Transformation|GetActorLocation) (Transformation|GetActorLocation (Variables|Default|GetDamageCauser)))) 2e+03) "root" false true)))

(event EventOnDamaged
  (params (Damage :type Float%20%28single-precision%29) (DamageCauser :type Actor%20Object%20Reference))
  (bind _hitmontageplayrate (Variables|Default|GetHitMontagePlayRate))
  ;[1 0.9532 0.1043] Damage Event
  (Utilities|FlowControl|Sequence
    (:then_0
      (Default|ReceiveMessageTag (Variables|Default|GetBP_BehaviorComponent) "NewEnumerator2"))
    (:then_1
      (bind _returnvalue (Class|AnimInstance|CalculateDirection (Components|SkeletalMesh|GetAnimInstance (Variables|Character|GetMesh)) (Math|Transform|InverseTransformDirection (Transformation|GetActorTransform) (- (Transformation|GetActorLocation) (Transformation|GetActorLocation DamageCauser))) (Transformation|GetActorRotation)))
      (Utilities|CalcDirection _returnvalue
        (:Front
          (Animation|PlayAnimMontage "/Game/Art/polygon/monster/Anim/z1_hit_front_Montage.z1_hit_front_Montage" _hitmontageplayrate "None"))
        (:Left
          (Animation|PlayAnimMontage "/Game/Art/polygon/monster/Anim/z1_hit_left_Montage.z1_hit_left_Montage" _hitmontageplayrate "None"))
        (:Right
          (Animation|PlayAnimMontage "/Game/Art/polygon/monster/Anim/z1_hit_right_Montage.z1_hit_right_Montage" _hitmontageplayrate "None"))
        (:Back
          (Animation|PlayAnimMontage "/Game/Art/polygon/monster/Anim/z1_hit_back_Montage.z1_hit_back_Montage" _hitmontageplayrate "None"))))))

(fn ConstructionScript
  (|CallParentFunction))