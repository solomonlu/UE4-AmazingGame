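; Skeleton knight monster Blueprint that handles hit reactions and death.
; On damage it sends a message tag to its behavior component and plays a front, left, right or back hit montage chosen from the angle to the damage causer.
; On death it adds a particle effect, then, if a controller is valid, unpossesses, notifies the behavior component and applies a physics impulse to the mesh away from the damage causer.
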(event EventOnDeath
  (bind _returnvalue (Pawn|GetController))
  (AddComponent|AddParticleSystemComponent false)
  (if (Utilities|IsValid _returnvalue)
    (Pawn|UnPossess _returnvalue)
    (Default|OnDeath (Variables|Default|GetBP_BehaviorComponent))
    (Class|SkeletalMeshComponent|AddImpulsetoAllBodiesBelow (Variables|Character|GetMesh) (* (Math|Vector|Normalize (- (Transformation|GetActorLocation) (Transformation|GetActorLocation (Variables|Default|GetDamageCauser)))) 2e+03) "root" false true)))

(event EventOnDamaged
  (params (Damage :type Float%20%28single-precision%29) (DamageCauser :type Actor%20Object%20Reference))
  (Utilities|FlowControl|Sequence
    (:then_0
      (Default|ReceiveMessageTag (Variables|Default|GetBP_BehaviorComponent) "NewEnumerator2"))
    (:then_1
      (bind _returnvalue (Class|AnimInstance|CalculateDirection (Components|SkeletalMesh|GetAnimInstance (Variables|Character|GetMesh)) (Math|Transform|InverseTransformDirection (Transformation|GetActorTransform) (- (Transformation|GetActorLocation) (Transformation|GetActorLocation DamageCauser))) (Transformation|GetActorRotation)))
      (Utilities|CalcDirection _returnvalue
        (:Front
          (Animation|PlayAnimMontage "/Game/Art/polygon/monster/Anim/z1_hit_front_Montage.z1_hit_front_Montage" 1.0 "None"))
        (:Left
          (Animation|PlayAnimMontage "/Game/Art/polygon/monster/Anim/z1_hit_left_Montage.z1_hit_left_Montage" 1.0 "None"))
        (:Right
          (Animation|PlayAnimMontage "/Game/Art/polygon/monster/Anim/z1_hit_right_Montage.z1_hit_right_Montage" 1.0 "None"))
        (:Back
          (Animation|PlayAnimMontage "/Game/Art/polygon/monster/Anim/z1_hit_back_Montage.z1_hit_back_Montage" 1.0 "None"))))))

(fn ConstructionScript
  (|CallParentFunction))