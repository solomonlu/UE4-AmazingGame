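; Base character for the spirits linked to the main character, with empty Attack and three Skill events for child classes to implement.
; Toggling control mode stops or restarts the AI controller's brain logic, and movement input applies only in Local mode.
; Changing spirit spawns the chosen subclass in place, transfers possession, updates the main character's SpiritRef and destroys itself.
; A looping timer from BeginPlay refreshes the main character reference.
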(event Custom|ToggleControlMode
  (bind _returnvalue (Pawn|GetController))
  (bind _asaicontroller (Utilities|Casting|CastToAIController _returnvalue))
  (bind _braincomponent (Variables|/Script/AIModule.AIController|GetBrainComponent _asaicontroller))
  ;[1 1 1] 目前只是AI和本地的切换
  (Variables|Default|SetControlMode (Utilities|Select :Index (Variables|Default|GetControlMode) :NewEnumerator0 "NewEnumerator1" :NewEnumerator1 "NewEnumerator0" :NewEnumerator2 "NewEnumerator0"))
  (switch Utilities|FlowControl|Switch|SwitchonESpiritControlMode (Variables|Default|GetControlMode)
    (:NewEnumerator0
      (Class|BrainComponent|RestartLogic _braincomponent))
    (:NewEnumerator1
      (AI|Logic|StopLogic _braincomponent ""))))

(event Custom|AddMoveInput
  (params (WorldVector :type Vector))
  (if (Utilities|Enum|Equal(Enum) (Variables|Default|GetControlMode) "NewEnumerator1")
    (Class|PawnMovementComponent|AddInputVector (Variables|Character|GetCharacterMovement) WorldVector false)))

(event Custom|Attack
  ;[1 1 1] Child implement
)

(event Custom|Skill1
  ;[1 1 1] Child implement
)

(event Custom|Skill2
  ;[1 1 1] Child implement
)

(event Custom|Skill3
  ;[1 1 1] Child implement
)

(event Custom|ChangeToAnotherSpirit
  (params (ChangeToSpiritCategory :type ESpiritCategory%20Enum :default "NewEnumerator0"))
  ;[1 1 1] 切换精灵
  (bind _returnvalue (Game|SpawnActorfromClass (Utilities|Select :Index ChangeToSpiritCategory :NewEnumerator0 "/Game/AmazingGame/Blueprints/Spirits/initialSpirit/BP_initialSpirit.BP_initialSpirit_C" :NewEnumerator1 "/Game/AmazingGame/Blueprints/Spirits/WaterSpirit/BP_WaterSpirit.BP_WaterSpirit_C" :NewEnumerator2 "/Game/AmazingGame/Blueprints/Spirits/FireSpirit/BP_FireSpirit.BP_FireSpirit_C" :NewEnumerator3 "/Game/AmazingGame/Blueprints/Spirits/ShadowSpirit/BP_ShadowSpirit.BP_ShadowSpirit_C") (Transformation|GetActorTransform) "Undefined" 0 0))
  (Pawn|Possess (Pawn|GetController) (.AsBP%20Spirit%20Base (Utilities|Casting|CastToBP_SpiritBase _returnvalue)))
  (Variables|/Game/AmazingGame/Blueprints/Character/BP_MainCharacter.BP_MainCharacter_C|SetSpiritRef (Variables|Default|GetMainCharacterRef) (.AsBP%20Spirit%20Base (Utilities|Casting|CastToBP_SpiritBase _returnvalue)))
  (Actor|DestroyActor))

(event EventBeginPlay
  (Utilities|Time|SetTimerbyFunctionName 0 "ChechMainCharacterRef" 1e+01 true)
  (CallFunction|ChechMainCharacterRef))

(fn ConstructionScript)

(fn ChechMainCharacterRef
  (bind _outactors (Actor|GetAllActorsOfClass "/Game/AmazingGame/Blueprints/Character/BP_MainCharacter.BP_MainCharacter_C"))
  (Variables|Default|SetMainCharacterRef (Utilities|Array|Get(acopy) _outactors)))