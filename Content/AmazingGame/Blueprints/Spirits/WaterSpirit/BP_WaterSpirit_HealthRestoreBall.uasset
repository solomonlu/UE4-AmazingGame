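; BP_WaterSpirit_HealthRestoreBall is a Water Spirit projectile that homes in on the main character and restores health on contact.
; On BeginPlay it finds the first BP_MainCharacter, targets its root component and activates ProjectileMovement as a homing projectile.
; Overlapping that character fires once, setting a short lifespan and healing by passing negative damage to ApplyDamage.
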(event EventBeginPlay
  (bind _projectilemovement (Variables|Default|GetProjectileMovement))
  (bind _outactors (Actor|GetAllActorsOfClass "/Game/AmazingGame/Blueprints/Character/BP_MainCharacter.BP_MainCharacter_C"))
  (if (> (Utilities|Array|Length _outactors) 0)
    (Variables|Default|SetMainCharacterRef (Utilities|Array|Get(acopy) _outactors))
    ;[1 1 1] Set homing
    (Variables|/Script/Engine.ProjectileMovementComponent|SetbIsHomingProjectile _projectilemovement true)
    (Variables|/Script/Engine.ProjectileMovementComponent|SetHomingTargetComponent _projectilemovement (Variables|/Script/Engine.Actor|GetRootComponent (Variables|Default|GetMainCharacterRef)))
    (Variables|/Script/Engine.ProjectileMovementComponent|SetHomingAccelerationMagnitude _projectilemovement 2e+03)
    (Components|Activation|SetActive _projectilemovement true false)))

(event Collision|EventActorBeginOverlap
  (params (OtherActor :type Actor%20Object%20Reference))
  (if (== OtherActor (Variables|Default|GetMainCharacterRef))
    (Utilities|FlowControl|DoOnce false
      (:Completed
        (Actor|SetLifeSpan 0.1)
        (Game|Damage|ApplyDamage (Variables|Default|GetMainCharacterRef) -25.0 0 0)))))

(fn ConstructionScript)