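; Fire spirit companion that carries out a melee attack and fireball skills, aimed by the main character's rotation.
; The normal attack plays a montage, and weapon overlaps damage monsters only while the SetValidAttack flag is on.
; Skill1 fires a three-ball fan, while Skill3 spawns a full ring of sixteen on its montage's FireBallAOE notify.
; Skill2 is an unimplemented placeholder.
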(event OnComponentBeginOverlap(WeaponCollision)
  (params (OverlappedComponent :type Primitive%20Component%20Object%20Reference) (OtherActor :type Actor%20Object%20Reference) (OtherComp :type Primitive%20Component%20Object%20Reference) (OtherBodyIndex :type Integer) (bFromSweep :type Boolean) (SweepResult :type Hit%20Result%20Structure%20%28by%20ref%29))
  ;[1 1 1] Normal Attack
  (if (Variables|Default|GetIsAttackValid)
    (bind _asbp_monster_base (Utilities|Casting|CastToBP_MonsterBase OtherActor))
    (Game|Damage|ApplyDamage _asbp_monster_base 5e+01 0 self)))

(event EventAttack
  ;[1 1 1] Normal Attack
  (Animation|Montage|PlayMontage (Variables|Character|GetMesh) "/Game/Art/anim/huojingling/huojingling_gongji1_Montage.huojingling_gongji1_Montage"))

(event EventSkill1
  (bind _maincharacterref (Variables|Default|GetMainCharacterRef))
  (bind _returnvalue (Transformation|GetActorRotation _maincharacterref))
  (for _index (range -1 1)
    (Game|SpawnActorfromClass "/Game/AmazingGame/Blueprints/Spirits/FireSpirit/BP_FireSpirit_AttackBall.BP_FireSpirit_AttackBall_C" (Math|Transform|MakeTransform (+ (Transformation|GetActorLocation) (* (Math|Vector|GetForwardVector (Math|Rotator|MakeRotator (.roll _returnvalue) (.pitch _returnvalue) (+ (* _index 22.5) (.yaw _returnvalue)))) 5e+01)) (Math|Rotator|MakeRotator (.roll _returnvalue) (.pitch _returnvalue) (+ (* _index 22.5) (.yaw _returnvalue))) "1,1,1") "Undefined" 0 0)))

(event EventSetValidAttack
  (params (IsValidAttack :type Boolean))
  ;[1 1 1] Normal Attack
  (Variables|Default|SetIsAttackValid IsValidAttack))

(event EventSkill2
  (Development|PrintString "TODO"))

(event EventSkill3
  (bind _maincharacterref (Variables|Default|GetMainCharacterRef))
  (bind _returnvalue (Transformation|GetActorRotation _maincharacterref))
  (bind _notifyname (Animation|Montage|PlayMontage (Variables|Character|GetMesh) "/Game/Art/anim/huojingling/huojingling_jineng_Montage.huojingling_jineng_Montage")
    (:OnNotifyBegin
      (if (Utilities|Name|Equal(Name) _notifyname "FireBallAOE")
        (for _index (range 0 15)
          (Game|SpawnActorfromClass "/Game/AmazingGame/Blueprints/Spirits/FireSpirit/BP_FireSpirit_AttackBall.BP_FireSpirit_AttackBall_C" (Math|Transform|MakeTransform (+ (Transformation|GetActorLocation) (* (Math|Vector|GetForwardVector (Math|Rotator|MakeRotator (.roll _returnvalue) (.pitch _returnvalue) (+ (* _index 22.5) (.yaw _returnvalue)))) 5e+01)) (Math|Rotator|MakeRotator (.roll _returnvalue) (.pitch _returnvalue) (+ (* _index 22.5) (.yaw _returnvalue))) "1,1,1") "Undefined" 0 0))))))

(fn ConstructionScript
  (|CallParentFunction))