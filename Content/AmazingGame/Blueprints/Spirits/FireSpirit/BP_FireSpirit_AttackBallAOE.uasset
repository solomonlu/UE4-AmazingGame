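; Fire Spirit area-of-effect attack actor that emits a radial burst of attack balls around itself, then destroys itself.
; After a short startup delay on BeginPlay, a LoopWithDelay macro repeatedly counts MaxAttack down to zero.
; Each pass uses the counter to step the yaw in 45-degree increments, spawning a BP_FireSpirit_AttackBall slightly out from the center, facing outward.
; A brief delay follows the last spawn before cleanup.
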(event EventBeginPlay
  (Utilities|FlowControl|Delay 1.2)
  (Utilities|LoopwithDelay (!= (Variables|Default|GetMaxAttack) 0) 0.25
    (:Body
      (bind _result (Math|Integer|DecrementInt (Variables|Default|GetMaxAttack))
        (:%20%20
          (Game|SpawnActorfromClass "/Game/AmazingGame/Blueprints/Spirits/FireSpirit/BP_FireSpirit_AttackBall.BP_FireSpirit_AttackBall_C" (Math|Transform|MakeTransform (+ (Transformation|GetActorLocation) (* (Math|Vector|GetForwardVector (Math|Rotator|MakeRotator 0.0 0.0 (* _result 45.0))) 5e+01)) (Math|Rotator|MakeRotator 0.0 0.0 (* _result 45.0)) "1,1,1") "Undefined" 0 0))))
    (:Completed
      (Utilities|FlowControl|Delay 0.8)
      (Actor|DestroyActor))))

(fn ConstructionScript)