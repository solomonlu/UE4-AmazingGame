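; BP_initialSpirit is the initial spirit, implementing a basic attack and three skills as spawned actors.
; Attack plays a montage and spawns an attack ball when its named notify begins, syncing it to the animation.
; The skills immediately spawn an AOE target, a spark and a wall.
; All spawns originate at the spirit but take the main character's rotation, with ball and wall offset along that forward direction.
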(event EventAttack
  (bind _maincharacterref (Variables|Default|GetMainCharacterRef))
  (bind _returnvalue (Transformation|GetActorRotation _maincharacterref))
  (bind _notifyname (Animation|Montage|PlayMontage (Variables|Character|GetMesh) "/Game/Art/anim/initialSpirit/SKM_1_XJL_Att_Montage.SKM_1_XJL_Att_Montage")
    (:OnNotifyBegin
      (if (Utilities|Name|Equal(Name) _notifyname "InitialSpiritAttackNotify")
        (Game|SpawnActorfromClass "/Game/AmazingGame/Blueprints/Spirits/initialSpirit/BP_InitialSpirit_AttackBall.BP_InitialSpirit_AttackBall_C" (Math|Transform|MakeTransform (+ (Transformation|GetActorLocation) (* (Math|Vector|GetForwardVector _returnvalue) 5e+01)) _returnvalue "1,1,1") "Undefined" 0 0)))))

(event EventSkill1
  (Game|SpawnActorfromClass "/Game/AmazingGame/Blueprints/Spirits/initialSpirit/BP_InitialSpirit_AOETarget.BP_InitialSpirit_AOETarget_C" (Math|Transform|MakeTransform (Transformation|GetActorLocation) (Transformation|GetActorRotation (Variables|Default|GetMainCharacterRef)) "1,1,1") "Undefined" 0 0))

(event EventSkill2
  (Game|SpawnActorfromClass "/Game/AmazingGame/Blueprints/Spirits/initialSpirit/BP_InitialSpirit_Spark.BP_InitialSpirit_Spark_C" (Math|Transform|MakeTransform (Transformation|GetActorLocation) (Transformation|GetActorRotation (Variables|Default|GetMainCharacterRef)) "1,1,1") "Undefined" 0 0))

(event EventSkill3
  (bind _maincharacterref (Variables|Default|GetMainCharacterRef))
  (bind _returnvalue (Transformation|GetActorRotation _maincharacterref))
  (Game|SpawnActorfromClass "/Game/AmazingGame/Blueprints/Spirits/initialSpirit/BP_InitialSpirit_Wall.BP_InitialSpirit_Wall_C" (Math|Transform|MakeTransform (+ (Transformation|GetActorLocation) (* (Math|Vector|GetForwardVector _returnvalue) 5e+01)) _returnvalue "1,1,1") "Undefined" 0 0))

(fn ConstructionScript
  (|CallParentFunction))