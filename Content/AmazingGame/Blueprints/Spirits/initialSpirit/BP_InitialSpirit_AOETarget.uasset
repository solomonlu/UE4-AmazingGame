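; BP_InitialSpirit_AOETarget is a short-lived target actor for the initial spirit's area attack, raining attack actors over its location.
; After a startup delay on BeginPlay, a LoopWithDelay macro repeatedly spawns BP_InitialSpirit_AOEAttack at random points in a box high above it, counting MaxAttack down to zero.
; The macro re-checks its condition after each short delay; on completion, the target waits briefly and destroys itself.
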(event EventBeginPlay
  (bind _returnvalue (Transformation|GetActorLocation))
  (Utilities|FlowControl|Delay 1.5)
  (Utilities|LoopwithDelay (!= (Variables|Default|GetMaxAttack) 0) 0.1
    (:Body
      (Math|Integer|DecrementInt (Variables|Default|GetMaxAttack)
        (:%20%20
          (Game|SpawnActorfromClass "/Game/AmazingGame/Blueprints/Spirits/initialSpirit/BP_InitialSpirit_AOEAttack.BP_InitialSpirit_AOEAttack_C" (Math|Transform|MakeTransform (Math|Random|RandomPointinBoundingBox (Math|Vector|MakeVector (.x _returnvalue) (.y _returnvalue) (+ (.z _returnvalue) 1e+03)) (Math|Vector|MakeVector 1e+02 1e+02 0.0)) "0, 0, 0" "1,1,1") "Undefined" 0 0))))
    (:Completed
      (Utilities|FlowControl|Delay 0.8)
      (Actor|DestroyActor))))

(fn ConstructionScript)