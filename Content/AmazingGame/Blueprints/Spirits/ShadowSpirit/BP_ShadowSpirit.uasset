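; Shadow spirit character with a three-hit melee combo and three skills.
; Attacks pressed mid-swing are buffered and continue the montage chain when CheckSaveAttack runs, until ResetCombo clears it.
; Weapon overlaps during the valid-attack window apply damage to BP_MonsterBase actors.
; Skills swap positions with the main character or spawn attached ShowTrap and Slomo actors.
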(event OnComponentBeginOverlap(WeaponCollision)
  (params (OverlappedComponent :type Primitive%20Component%20Object%20Reference) (OtherActor :type Actor%20Object%20Reference) (OtherComp :type Primitive%20Component%20Object%20Reference) (OtherBodyIndex :type Integer) (bFromSweep :type Boolean) (SweepResult :type Hit%20Result%20Structure%20%28by%20ref%29))
  (if (Variables|Default|GetIsAttackValid)
    (bind _asbp_monster_base (Utilities|Casting|CastToBP_MonsterBase OtherActor))
    (Game|Damage|ApplyDamage _asbp_monster_base 25.0 0 self)))

(event EventAttack
  (bind _mesh (Variables|Character|GetMesh))
  (bind _returnvalue (Components|SkeletalMesh|GetAnimInstance _mesh))
  ;[1 1 1] Normal Attack
  (if (Variables|Default|GetIsAttacking)
    (Variables|Default|SetSaveAttack true)
    (else
      (Variables|Default|SetIsAttacking true)
      (switch int (Variables|Default|GetComboCounter)
        (:0
          (Variables|Default|SetComboCounter 1)
          (Animation|Montage|MontagePlay _returnvalue "/Game/Art/polygon/PolygonDungeons/Anim/swordAnimset/Root/Attack_16_Montage.Attack_16_Montage" 1.0 "MontageLength" 0.0 true))
        (:1
          (Variables|Default|SetComboCounter 2)
          (Animation|Montage|MontagePlay _returnvalue "/Game/Art/polygon/PolygonDungeons/Anim/swordAnimset/Root/Attack_09_Montage.Attack_09_Montage" 1.0 "MontageLength" 0.0 true))
        (:2
          (Variables|Default|SetComboCounter 0)
          (Animation|Montage|MontagePlay _returnvalue "/Game/Art/polygon/PolygonDungeons/Anim/swordAnimset/Root/Attack_17_Montage.Attack_17_Montage" 1.0 "MontageLength" 0.0 true))))))

(event EventSkill1
  (CallFunction|SwapActorLocation (Variables|Default|GetMainCharacterRef) self))

(event EventSetValidAttack
  (params (IsValidAttack :type Boolean))
  (Variables|Default|SetIsAttackValid IsValidAttack))

(event EventSkill2
  (bind _returnvalue (Game|SpawnActorfromClass "/Game/AmazingGame/Blueprints/Spirits/ShadowSpirit/BP_ShadowSpirit_ShowTrap.BP_ShadowSpirit_ShowTrap_C" (Math|Transform|MakeTransform "0, 0, 0" "0, 0, 0" "1,1,1") "Undefined" 0 0))
  (Transformation|AttachActorToActor _returnvalue self "None" "KeepRelative" "KeepRelative" "KeepRelative" false))

(event EventResetCombo
  ;[1 1 1] Normal Attack
  (Variables|Default|SetComboCounter 0)
  (Variables|Default|SetSaveAttack false)
  (Variables|Default|SetIsAttacking false))

(event EventCheckSaveAttack
  (bind _mesh (Variables|Character|GetMesh))
  (bind _returnvalue (Components|SkeletalMesh|GetAnimInstance _mesh))
  ;[1 1 1] Normal Attack
  (if (Variables|Default|GetSaveAttack)
    (Variables|Default|SetSaveAttack false)
    (switch int (Variables|Default|GetComboCounter)
      (:0
        (Variables|Default|SetComboCounter 1)
        (Animation|Montage|MontagePlay _returnvalue "/Game/Art/polygon/PolygonDungeons/Anim/swordAnimset/Root/Attack_16_Montage.Attack_16_Montage" 1.0 "MontageLength" 0.0 true))
      (:1
        (Variables|Default|SetComboCounter 2)
        (Animation|Montage|MontagePlay _returnvalue "/Game/Art/polygon/PolygonDungeons/Anim/swordAnimset/Root/Attack_09_Montage.Attack_09_Montage" 1.0 "MontageLength" 0.0 true))
      (:2
        (Variables|Default|SetComboCounter 0)
        (Animation|Montage|MontagePlay _returnvalue "/Game/Art/polygon/PolygonDungeons/Anim/swordAnimset/Root/Attack_17_Montage.Attack_17_Montage" 1.0 "MontageLength" 0.0 true)))))

(event EventSkill3
  (bind _returnvalue (Game|SpawnActorfromClass "/Game/AmazingGame/Blueprints/Spirits/ShadowSpirit/BP_ShadowSpirit_Slomo.BP_ShadowSpirit_Slomo_C" (Math|Transform|MakeTransform "0, 0, 0" "0, 0, 0" "1,1,1") "Undefined" 0 0))
  (Transformation|AttachActorToActor _returnvalue self "None" "KeepRelative" "KeepRelative" "KeepRelative" false))

(fn ConstructionScript
  (|CallParentFunction))

(fn SwapActorLocation
  (params (Actor1 :type Actor%20Object%20Reference) (Actor2 :type Actor%20Object%20Reference))
  (Utilities|FlowControl|Sequence
    (:then_0
      (LocalVariables|SetTempLocation (Transformation|GetActorLocation Actor1)))
    (:then_1
      (Transformation|SetActorLocation Actor1 (Transformation|GetActorLocation Actor2) false false))
    (:then_2
      (Transformation|SetActorLocation Actor2 (LocalVariables|GetTempLocation) false false))))