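; BP_SpiritHeadPortrait is a spirit head portrait that displays the mesh matching the main character's current spirit category.
; BeginPlay caches the first BP_MainCharacter found in the level.
; Every Tick it hides the Initial, Water, Fire and Shadow meshes, then unhides the one selected by that character's SpiritRef category, polling rather than reacting to change events.
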(event EventBeginPlay
  (bind _outactors (Actor|GetAllActorsOfClass "/Game/AmazingGame/Blueprints/Character/BP_MainCharacter.BP_MainCharacter_C"))
  (Variables|Default|SetMainCharacterRef (Utilities|Array|Get(acopy) _outactors)))

(event EventTick
  (params (DeltaSeconds :type Float%20%28single-precision%29))
  (Development|SetHiddeninGame (Variables|Default|GetWaterMesh) true false)
  (Development|SetHiddeninGame (Utilities|Select :Index (Variables|/Game/AmazingGame/Blueprints/Spirits/BP_SpiritBase.BP_SpiritBase_C|GetSpiritCategory (Variables|/Game/AmazingGame/Blueprints/Character/BP_MainCharacter.BP_MainCharacter_C|GetSpiritRef (Variables|Default|GetMainCharacterRef))) :NewEnumerator0 (Variables|Default|GetInitialMesh) :NewEnumerator1 (Variables|Default|GetWaterMesh) :NewEnumerator2 (Variables|Default|GetFireMesh) :NewEnumerator3 (Variables|Default|GetShadowMesh)) false false))

(fn ConstructionScript)