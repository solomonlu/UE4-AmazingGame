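; BP_Trap_RockFallenArea is a trigger-box trap that rains rocks on the main character while they stay inside.
; Entering starts a timeline whose event track spawns BP_Trap_RockFallen at random points overhead, using a suggested projectile velocity to lob each at the player's current position.
; Leaving stops and resets the timeline, while lasting until it finishes disables box collision, fires OnSuccess after a delay and destroys the trap.
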(event OnComponentBeginOverlap(Box)
  (params (OverlappedComponent :type Primitive%20Component%20Object%20Reference) (OtherActor :type Actor%20Object%20Reference) (OtherComp :type Primitive%20Component%20Object%20Reference) (OtherBodyIndex :type Integer) (bFromSweep :type Boolean) (SweepResult :type Hit%20Result%20Structure%20%28by%20ref%29))
  (bind _asbp_main_character (Utilities|Casting|CastToBP_MainCharacter OtherActor))
  (Variables|Default|SetMainCharacterRef _asbp_main_character)
  (Utilities|FlowControl|DoOnce false
    (:Completed
      (Timeline|TimelineRockFallen PlayFromStart
        (:Finished
          (Collision|SetCollisionResponsetoAllChannels (Variables|Default|GetBox) "ECR_Ignore")
          (Utilities|FlowControl|Delay 5.0)
          (Default|CallOnSuccess)
          (Development|PrintString "Success")
          (Actor|DestroyActor))
        (:RockFallenEvent
          (bind _output_get (Variables|Default|SetTempSpawnRockLocation (+ (Math|Random|RandomPointinBoundingBox (Transformation|GetActorLocation) (* (Variables|/Script/Engine.BoxComponent|GetBoxExtent (Variables|Default|GetBox)) 1.5)) "0, 0,1000.000000")))
          (bind (_tossvelocity _returnvalue) (Class|GameplayStatics|BlueprintSuggestProjectileVelocity _output_get (Transformation|GetActorLocation (Variables|Default|GetMainCharacterRef)) 5e+02 -9.8e+02 "DoNotTrace" 0.0 true false))
          (if _returnvalue
            (Game|SpawnActorfromClass "/Game/AmazingGame/Blueprints/Trap/BP_Trap_RockFallen.BP_Trap_RockFallen_C" (Math|Transform|MakeTransform (Variables|Default|GetTempSpawnRockLocation) "0, 0, 0" "1,1,1") "Undefined" 0 _tossvelocity 0)))))))

(event OnComponentEndOverlap(Box)
  (params (OverlappedComponent :type Primitive%20Component%20Object%20Reference) (OtherActor :type Actor%20Object%20Reference) (OtherComp :type Primitive%20Component%20Object%20Reference) (OtherBodyIndex :type Integer))
  (Utilities|Casting|CastToBP_MainCharacter OtherActor)
  (Utilities|FlowControl|Sequence
    (:then_0
      (Timeline|TimelineRockFallen Stop
        (:Finished
          (Collision|SetCollisionResponsetoAllChannels (Variables|Default|GetBox) "ECR_Ignore")
          (Utilities|FlowControl|Delay 5.0)
          (Default|CallOnSuccess)
          (Development|PrintString "Success")
          (Actor|DestroyActor))
        (:RockFallenEvent
          (bind _output_get (Variables|Default|SetTempSpawnRockLocation (+ (Math|Random|RandomPointinBoundingBox (Transformation|GetActorLocation) (* (Variables|/Script/Engine.BoxComponent|GetBoxExtent (Variables|Default|GetBox)) 1.5)) "0, 0,1000.000000")))
          (bind (_tossvelocity _returnvalue) (Class|GameplayStatics|BlueprintSuggestProjectileVelocity _output_get (Transformation|GetActorLocation (Variables|Default|GetMainCharacterRef)) 5e+02 -9.8e+02 "DoNotTrace" 0.0 true false))
          (if _returnvalue
            (Game|SpawnActorfromClass "/Game/AmazingGame/Blueprints/Trap/BP_Trap_RockFallen.BP_Trap_RockFallen_C" (Math|Transform|MakeTransform (Variables|Default|GetTempSpawnRockLocation) "0, 0, 0" "1,1,1") "Undefined" 0 _tossvelocity 0)))))
    (:then_1
      (Timeline|TimelineRockFallen SetNewTime))
    (:then_2
      (Utilities|FlowControl|DoOnce false) ; enters at Reset
    )))

(fn ConstructionScript)