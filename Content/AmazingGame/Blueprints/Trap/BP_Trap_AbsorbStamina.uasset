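; A trap that drains stamina from the main character while it is inside the Box trigger.
; Overlap by the character's root component stores a reference, starts a gate and delay loop removing stamina every half second, and calls OnPlayerIntoArea.
; End overlap only clears the reference: the gate is never closed, so the loop keeps running and skips the drain while the reference is invalid.
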(event OnComponentBeginOverlap(Box)
  (params (OverlappedComponent :type Primitive%20Component%20Object%20Reference) (OtherActor :type Actor%20Object%20Reference) (OtherComp :type Primitive%20Component%20Object%20Reference) (OtherBodyIndex :type Integer) (bFromSweep :type Boolean) (SweepResult :type Hit%20Result%20Structure%20%28by%20ref%29))
  (bind _asbp_main_character (Utilities|Casting|CastToBP_MainCharacter (Components|GetOwner OtherComp)))
  (if (== (Variables|/Script/Engine.Actor|GetRootComponent _asbp_main_character) OtherComp)
    (Variables|Default|SetMainCharacterRef _asbp_main_character)
    (Utilities|FlowControl|Sequence
      (:then_0
        (goto _label Open))
      (:then_1
        (Utilities|FlowControl|Gate true :!label _label
          (:Exit
            (Utilities|IsValid (Variables|Default|GetMainCharacterRef)
              (:Is%20Valid
                (Default|AddStamina (Variables|Default|GetMainCharacterRef) -2e+01))
              (:Is%20Not%20Valid
                _))
            (Utilities|FlowControl|Delay 0.5)
            (goto _label))))
      (:then_2
        (Default|CallOnPlayerIntoArea)))))

(event OnComponentEndOverlap(Box)
  (params (OverlappedComponent :type Primitive%20Component%20Object%20Reference) (OtherActor :type Actor%20Object%20Reference) (OtherComp :type Primitive%20Component%20Object%20Reference) (OtherBodyIndex :type Integer))
  (bind _asbp_main_character (Utilities|Casting|CastToBP_MainCharacter (Components|GetOwner OtherComp)))
  (if (== (Variables|/Script/Engine.Actor|GetRootComponent _asbp_main_character) OtherComp)
    (Variables|Default|SetMainCharacterRef 0)))

(fn ConstructionScript)