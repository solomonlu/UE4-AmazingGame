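; BP_Trap_Spear is a floor spear trap that springs once and then stays active, damaging characters standing in it.
; The first overlap of ActiveBox plays a timeline that raises the spear mesh, then sets IsActive.
; While active, Tick damages every Character overlapping the box, using a Gate and Delay to limit hits to a half-second interval.
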(event OnComponentBeginOverlap(ActiveBox)
  (params (OverlappedComponent :type Primitive%20Component%20Object%20Reference) (OtherActor :type Actor%20Object%20Reference) (OtherComp :type Primitive%20Component%20Object%20Reference) (OtherBodyIndex :type Integer) (bFromSweep :type Boolean) (SweepResult :type Hit%20Result%20Structure%20%28by%20ref%29))
  (Utilities|FlowControl|DoOnce false
    (:Completed
      (bind _lerp (Timeline|TimelineActive PlayFromStart)
        (:Update
          (Transformation|SetRelativeLocation (Variables|Default|GetSM_Prop_Trap_Spears_01) (Math|Vector|MakeVector 0.0 0.0 (Math|Float|Lerp -2e+02 0.0 _lerp)) false false))
        (:Finished
          (Variables|Default|SetIsActive true))))))

(event EventTick
  (params (DeltaSeconds :type Float%20%28single-precision%29))
  (if (Variables|Default|GetIsActive)
    (Utilities|FlowControl|Gate false :!label _label
      (:Exit
        (Utilities|FlowControl|Sequence
          (:then_0
            (goto _label Close))
          (:then_1
            (for _array_element (Collision|GetOverlappingActors (Variables|Default|GetActiveBox) "/Script/Engine.Character" :!class /Script/Engine.PrimitiveComponent)
              (Game|Damage|ApplyDamage _array_element 1e+02 0 self))
            (Utilities|FlowControl|Delay 0.5)
            (goto _label Open)))))))

(fn ConstructionScript)