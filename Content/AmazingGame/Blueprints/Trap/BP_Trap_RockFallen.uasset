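; BP_Trap_RockFallen is a rock trap projectile that damages the main character.
; Its construction script randomizes the pebble mesh rotation and feeds a Velocity variable into ProjectileMovement.
; The Sphere applies damage once when it overlaps BP_MainCharacter and destroys the actor on a hit.
; A shatter-effect emitter spawn is present but unconnected, so it never runs.
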(event OnComponentBeginOverlap(Sphere)
  (params (OverlappedComponent :type Primitive%20Component%20Object%20Reference) (OtherActor :type Actor%20Object%20Reference) (OtherComp :type Primitive%20Component%20Object%20Reference) (OtherBodyIndex :type Integer) (bFromSweep :type Boolean) (SweepResult :type Hit%20Result%20Structure%20%28by%20ref%29))
  (bind _asbp_main_character (Utilities|Casting|CastToBP_MainCharacter OtherActor))
  (Utilities|FlowControl|DoOnce false
    (:Completed
      (Game|Damage|ApplyDamage _asbp_main_character 25.0 0 0))))

(event OnComponentHit(Sphere)
  (params (HitComponent :type Primitive%20Component%20Object%20Reference) (OtherActor :type Actor%20Object%20Reference) (OtherComp :type Primitive%20Component%20Object%20Reference) (NormalImpulse :type Vector :default "0, 0, 0") (Hit :type Hit%20Result%20Structure%20%28by%20ref%29))
  (Utilities|FlowControl|DoOnce false
    (:Completed
      (Actor|DestroyActor))))

(fn ConstructionScript
  (Transformation|SetRelativeRotation (Variables|Default|GetSM_Env_Rock_Pebble_01) (Math|Random|RandomRotator true) false false)
  (Variables|/Script/Engine.MovementComponent|SetVelocity (Variables|Default|GetProjectileMovement) (Variables|Default|GetVelocity)))