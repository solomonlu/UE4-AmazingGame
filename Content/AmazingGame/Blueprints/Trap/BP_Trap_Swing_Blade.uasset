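; Swinging blade trap that deals heavy damage to any Character whose root component overlaps the blade mesh.
; A timeline started on BeginPlay drives the blade's pitch back and forth with swept relative rotation.
; Show and unshow events toggle the "Trap" material scalar on the blade to change its appearance.
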(event OnComponentBeginOverlap(SM_Prop_Trap_Swing_Blade_01)
  (params (OverlappedComponent :type Primitive%20Component%20Object%20Reference) (OtherActor :type Actor%20Object%20Reference) (OtherComp :type Primitive%20Component%20Object%20Reference) (OtherBodyIndex :type Integer) (bFromSweep :type Boolean) (SweepResult :type Hit%20Result%20Structure%20%28by%20ref%29))
  (bind _ascharacter (Utilities|Casting|CastToCharacter (Components|GetOwner OtherComp)))
  (if (== (Variables|/Script/Engine.Actor|GetRootComponent _ascharacter) OtherComp)
    (Game|Damage|ApplyDamage _ascharacter 1e+02 0 self)))

(event EventOnShowTrap
  (Rendering|Material|SetScalarParameterValueonMaterials (Variables|Default|GetSM_Prop_Trap_Swing_Blade_01) "Trap" 1.0))

(event EventOnUnshowTrap
  (Rendering|Material|SetScalarParameterValueonMaterials (Variables|Default|GetSM_Prop_Trap_Swing_Blade_01) "Trap" 0.0))

(event EventBeginPlay
  (Components|Timeline|PlayfromStart (Variables|Default|GetTimelineSwing)))

(fn ConstructionScript)