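; Trap area that summons random skeleton enemies inside its box and reports success once all of them are dead.
; Start destroys earlier spawns, then plays a timeline whose events each spawn one of four skeleton types at a random point and yaw.
; After the timeline finishes, Tick polls the living count.
; At zero, a DoOnce makes the box ignore collision, then calls OnSuccess after a short delay.
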(event Custom|Start
  (bind _returnvalue (Transformation|GetActorLocation))
  (bind _returnvalue_2 (Math|Random|RandomFloatinRange 0.0 3.6e+02))
  (bind _box (Variables|Default|GetBox))
  (bind _boxextent (Variables|/Script/Engine.BoxComponent|GetBoxExtent _box))
  (bind _returnvalue_3 (Math|Vector|MakeVector (.x _boxextent) (.y _boxextent) 0.0))
  (bind _returnvalue_4 (* _returnvalue_3 0.5))
  (bind _returnvalue_5 (Math|Random|RandomPointinBoundingBox _returnvalue _returnvalue_4))
  (for _array_element (Variables|Default|GetSpawnedSkeletons)
    (Utilities|IsValid _array_element
      (:Is%20Valid
        (Actor|DestroyActor _array_element))))
  (Utilities|Array|Clear (Variables|Default|GetSpawnedSkeletons))
  (Variables|Default|SetIsStartCheck false)
  (Timeline|TimelineSummonSkeleton PlayFromStart
    (:Finished
      (Variables|Default|SetIsStartCheck true))
    (:SummonSkeletonEvent
      (Math|Integer|IncrementInt (Variables|Default|GetSpawnedSkeleton)
        (:%20%20
          (switch int (Math|Random|RandomIntegerinRange 0 3)
            (:0
              (bind _returnvalue_6 (Game|SpawnActorfromClass "/Game/AmazingGame/Blueprints/Monster/Skeleton/BP_SkeletonKight.BP_SkeletonKight_C" (Math|Transform|MakeTransform _returnvalue_5 (Math|Rotator|MakeRotator 0.0 0.0 _returnvalue_2) "1,1,1") "Undefined" 0 "NewEnumerator1" true 0))
              (Utilities|Array|AddUnique (Variables|Default|GetSpawnedSkeletons) _returnvalue_6))
            (:1
              (bind _returnvalue_7 (Game|SpawnActorfromClass "/Game/AmazingGame/Blueprints/Monster/Skeleton/BP_SkeletonSlave.BP_SkeletonSlave_C" (Math|Transform|MakeTransform _returnvalue_5 (Math|Rotator|MakeRotator 0.0 0.0 _returnvalue_2) "1,1,1") "Undefined" 0 "NewEnumerator1" true 0))
              (Utilities|Array|AddUnique (Variables|Default|GetSpawnedSkeletons) _returnvalue_7))
            (:2
              (bind _returnvalue_8 (Game|SpawnActorfromClass "/Game/AmazingGame/Blueprints/Monster/Skeleton/BP_SkeletonSoldier1.BP_SkeletonSoldier1_C" (Math|Transform|MakeTransform _returnvalue_5 (Math|Rotator|MakeRotator 0.0 0.0 _returnvalue_2) "1,1,1") "Undefined" 0 "NewEnumerator1" true 0))
              (Utilities|Array|AddUnique (Variables|Default|GetSpawnedSkeletons) _returnvalue_8))
            (:3
              (bind _returnvalue_9 (Game|SpawnActorfromClass "/Game/AmazingGame/Blueprints/Monster/Skeleton/BP_SkeletonSoldier2.BP_SkeletonSoldier2_C" (Math|Transform|MakeTransform _returnvalue_5 (Math|Rotator|MakeRotator 0.0 0.0 _returnvalue_2) "1,1,1") "Undefined" 0 "NewEnumerator1" true 0))
              (Utilities|Array|AddUnique (Variables|Default|GetSpawnedSkeletons) _returnvalue_9))))))))

(event EventTick
  (params (DeltaSeconds :type Float%20%28single-precision%29))
  (if (Variables|Default|GetIsStartCheck)
    (if (== (CallFunction|CheckAliveSkeleton) 0)
      (Utilities|FlowControl|DoOnce false
        (:Completed
          (Collision|SetCollisionResponsetoAllChannels (Variables|Default|GetBox) "ECR_Ignore")
          (Utilities|FlowControl|Delay 2.0)
          (Default|CallOnSuccess)
          (Development|PrintString "Success"))))))

(fn ConstructionScript)

(fn CheckAliveSkeleton
  (for _array_element (Variables|Default|GetSpawnedSkeletons)
    (Utilities|IsValid _array_element
      (:Is%20Valid
        (if (> (Variables|/Game/AmazingGame/Blueprints/Monster/BP_MonsterBase.BP_MonsterBase_C|GetCurrentHealth _array_element) 0.0)
          (Math|Integer|IncrementInt (LocalVariables|GetAliveSkeleton))))))
  (return (LocalVariables|GetAliveSkeleton)))